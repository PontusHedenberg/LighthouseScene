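; An actor that moves a cargo ship mesh along a spline, with a periodic horn sound.
; A timeline started on BeginPlay drives an alpha that sets the ship's world location and rotation by spline distance, at a fixed scale.
; Timeline updates also feed a delayed DoOnce that plays the attached horn and resets after a further delay.
; When the timeline finishes, it waits, then restarts from the beginning if the alpha passes a threshold check.
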(event EventBeginPlay
  (bind _spline (Variables|Default|GetSpline))
  (bind _cargoship (Variables|Default|GetCargoShip))
  (bind _animationalpha (Timeline|Timeline_0 PlayFromStart)
    (:Update
      (Transformation|SetWorldTransform _cargoship (Math|Transform|MakeTransform (Spline|GetLocationatDistanceAlongSpline _spline (* _animationalpha (Spline|GetSplineLength _spline)) "World") (Spline|GetRotationatDistanceAlongSpline _spline (* _animationalpha (Spline|GetSplineLength _spline)) "World") "7.000000,7.000000,7.000000") false false)
      (Utilities|FlowControl|Delay 2e+01)
      (Utilities|FlowControl|DoOnce false :!label _label
        (:Completed
          (Audio|SpawnSoundAttached "/Game/ShipHorn.ShipHorn" _cargoship "None" "0, 0, 0" "0, 0, 0" "KeepRelativeOffset" false 0.1 1.0 0.0 0 0)
          (Utilities|FlowControl|Delay 47.0)
          (goto _label Reset))))
    (:Finished
      (if (<= _animationalpha 4e+01)
        (Utilities|FlowControl|Delay 27.0)
        (Timeline|Timeline_0 PlayFromStart)))))

(event Collision|EventActorBeginOverlap
  (params (OtherActor :type Actor%20Object%20Reference)))

(event EventTick
  (params (DeltaSeconds :type Float%20%28single-precision%29)))

(fn ConstructionScript)